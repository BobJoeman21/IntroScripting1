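; BP_FPSChar is a first-person character with Enhanced Input look and move, likely a learning exercise.
; BeginPlay adds the mapping context, look drives controller yaw and pitch, and move applies actor-relative movement while printing a debug "Hello".
; The construction script looks up EnumTest in EnumTestMap and uses the resulting struct to set an added static mesh and the particle template, and print a spawn message.
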(event `EnhancedInput|/Game/Blueprints/Week05/Input/IA_FPSLook`
  (params (ActionValue :type "Vector2D Structure") (ElapsedSeconds :type "Float (double-precision)") (TriggeredSeconds :type "Float (double-precision)") (InputAction :type "InputAction Object Reference" :default "/Game/Blueprints/Week05/Input/IA_FPSLook.IA_FPSLook"))
  (:`Triggered`
    (`self.AddControllerYawInput` ActionValue_X)
    (`self.AddControllerPitchInput` ActionValue_Y)))

(event `EnhancedInput|/Game/Blueprints/Week05/Input/IA_FPSMove`
  (params (ActionValue :type "Vector2D Structure") (ElapsedSeconds :type "Float (double-precision)") (TriggeredSeconds :type "Float (double-precision)") (InputAction :type "InputAction Object Reference" :default "/Game/Blueprints/Week05/Input/IA_FPSMove.IA_FPSMove"))
  (:`Triggered`
    (`self.AddMovementInput` (`self.GetActorRightVector`) ActionValue_X)
    (`self.AddMovementInput` (`self.GetActorForwardVector`) ActionValue_Y)
    (`KismetSystemLibrary.PrintText` "Hello")))

(event `self.ReceiveBeginPlay`
  (`EnhancedInputSubsystemInterface.AddMappingContext` (pcsubsystem `EnhancedInputLocalPlayerSubsystem` (`GameplayStatics.GetPlayerController` 0)) "/Game/Blueprints/Week05/Input/IA_FPSMap.IA_FPSMap" 0 (struct)))

(fn `UserConstructionScript`
  (bind _value (`BlueprintMapLibrary.Map_Find` (`self.EnumTestMap`) (`self.EnumTest`)))
  (bind _returnvalue (`AddComponent|NODE_AddStaticMeshComponent-0`))
  (`StaticMeshComponent.SetStaticMesh` _returnvalue (break `/Game/Blueprints/Week05/StructTest` _value))
  (`ParticleSystemComponent.SetTemplate` (`self.ParticleSystem`) (`.StructEffect_9_5463E9844D12B23BBAB003A173DEF4D1` (break `/Game/Blueprints/Week05/StructTest` _value)))
  (`KismetSystemLibrary.PrintString` (`.StructSpawnMessage_8_DC7C02194EAB992EDF39ED868548F7AE` (break `/Game/Blueprints/Week05/StructTest` _value))))