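; BP_Attack is an actor that performs a single attack when play begins and presents it as strong or weak.
; Attack optionally randomizes Strength, then a helper function derives the attack value from it with a linear formula.
; A threshold on that value picks which particle effect and sound to play, and the tier and number are printed.
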(event `self.ReceiveBeginPlay`
  (`self.Attack`))

(event `Attack`
  (if (`self.Randomize Str`)
    (bind _output_get (set `self.Strength` (`KismetMathLibrary.RandomIntegerInRange` 1 10))))
  (bind _attackval (`self.Calculate Attack` _output_get))
  (if (>= _attackval 40)
    (`KismetSystemLibrary.PrintString` "STRONG ATTACK")
    (`ActorComponent.Activate` (`self.StrongPart`) true)
    (`AudioComponent.Play` (`self.StrongSound`) 0.0)
    (else
      (`KismetSystemLibrary.PrintString` "WEAK ATTACK")
      (`ActorComponent.Activate` (`self.WeakPart`) true)
      (`AudioComponent.Play` (`self.WeakSound`) 0.0)))
  (`KismetSystemLibrary.PrintText` (`KismetTextLibrary.Conv_IntToText` _attackval)))

(fn `Calculate Attack`
  (params (StrengthVal :type Integer))
  (returns (AttackVal :type Integer))
  (return (+ (* StrengthVal 5) 10)))

(fn `UserConstructionScript`)