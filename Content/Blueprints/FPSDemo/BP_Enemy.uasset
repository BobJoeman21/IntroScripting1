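; BP_Enemy is a damageable FPS demo enemy that chases the player once activated.
; Damage lowers its health and updates a widget health bar, and at zero it spawns BP_Explosion and destroys itself.
; Tick feeds a start-closed DoOnce that Activate opens, issuing AI Move To toward the player's current location and resetting on success or failure to keep the chase going.
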(event `self.ReceiveAnyDamage`
  (params (Damage :type "Float (single-precision)") (DamageType :type "DamageType Object Reference") (InstigatedBy :type "Controller Object Reference") (DamageCauser :type "Actor Object Reference"))
  (`KismetSystemLibrary.PrintString` (`KismetStringLibrary.Concat_StrStr` "Took " (`KismetStringLibrary.Conv_DoubleToString` Damage) " Damage"))
  (bind _output_get (set `self.CurrentHealthValue` (- (`self.CurrentHealthValue`) Damage)))
  (`/Game/Blueprints/FPSDemo/BP_Healthbar.ChangeValue` (`self.As BP Healthbar`) (/ _output_get (`self.MaxHealthValue`)))
  (if (<= (`self.CurrentHealthValue`) 0.0)
    (`|SpawnActorFromClass` "/Game/Blueprints/Week03/BP_Explosion.BP_Explosion_C" (`self.GetTransform`) "Undefined" "MultiplyWithRoot" null null)
    (`self.K2_DestroyActor`)))

(event `self.ReceiveBeginPlay`
  (bind _asbp_healthbar (cast `/Game/Blueprints/FPSDemo/BP_Healthbar` (`WidgetComponent.GetUserWidgetObject` (`self.Widget`))))
  (bind _output_get (set `self.As BP Healthbar` _asbp_healthbar))
  (`/Game/Blueprints/FPSDemo/BP_Healthbar.ChangeValue` _output_get (/ (`self.CurrentHealthValue`) (`self.MaxHealthValue`))))

(event `self.ReceiveTick`
  (params (DeltaSeconds :type "Float (single-precision)"))
  (`/Engine/EditorBlueprintResources/StandardMacros.DoOnce` true :!label _label
    (:`Completed`
      (`|AIMoveTo` self (`self.K2_GetActorLocation` (`GameplayStatics.GetPlayerCharacter` 0)) null 0.2
        (:`OnSuccess`
          (goto _label :!via `Reset`))
        (:`OnFail`
          (goto _label :!via `Reset`))))))

(event `Activate`
  (goto _label :!via `Reset`))

(fn `UserConstructionScript`)