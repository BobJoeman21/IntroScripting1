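; BP_Door is an interactable door that swings 90 degrees open or closed and can require a colored key.
; Interacting while locked spends a matching key from the player's NumberofKeys map, updates the UI and unlocks the door, or prints a no-keys message.
; A FlipFlop plays or reverses the DoorOpen timeline, which lerps the door's yaw.
; The construction script sets a locked door's material to match its key color.
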(event `self.ReceiveBeginPlay`
  (bind (_returnvalue_roll _returnvalue_pitch _returnvalue_yaw) (`KismetMathLibrary.BreakRotator` (`SceneComponent.K2_GetComponentRotation` (`self.Door`))))
  (set `self.StartYaw` _returnvalue_yaw)
  (set `self.GoalYaw` (+ _returnvalue_yaw 90.0)))

(event `Interacted`
  (params (PlayerChar :type "/Game/FirstPersonAssets/FirstPerson/Blueprints/BP_FirstPersonCharacter Object Reference") (UI :type "/Game/Blueprints/FPSDemo/BP_FPSHUD Object Reference"))
  (bind _doorcolor (`self.DoorColor`))
  (bind _numberofkeys (`/Game/FirstPersonAssets/FirstPerson/Blueprints/BP_FirstPersonCharacter.NumberofKeys` PlayerChar))
  (bind _value (`BlueprintMapLibrary.Map_Find` _numberofkeys _doorcolor))
  (if (`self.IsLocked`)
    (if (> _value 0)
      (`BlueprintMapLibrary.Map_Add` _numberofkeys _doorcolor (- _value 1))
      (`/Game/Blueprints/FPSDemo/BP_FPSHUD.UpdateKey` UI _doorcolor _value)
      (set `self.IsLocked` false)
      ;[1 1 1] OpenDoor
      (`/Engine/EditorBlueprintResources/StandardMacros.FlipFlop` :!label _label
        (:`A`
          (bind (_direction _lerpprog) (`Timeline|DoorOpen` :!label _label_2)
            (:`Update`
              (`SceneComponent.K2_SetWorldRotation` (`self.Door`) (`KismetMathLibrary.MakeRotator` 0.0 0.0 (`KismetMathLibrary.Lerp` (`self.StartYaw`) (`self.GoalYaw`) _lerpprog)) false false))))
        (:`B`
          (goto _label_2 :!via `Reverse`)))
      (else
        (`KismetSystemLibrary.PrintText` "NoKeys")))
    (else
      (goto _label))))

(fn `UserConstructionScript`
  (bind _door (`self.Door`))
  (if (`self.IsLocked`)
    (switch `/Game/Blueprints/FPSDemo/EKeyColor` (`self.DoorColor`)
      (:`NewEnumerator0`
        (`PrimitiveComponent.SetMaterial` _door 0 "/Game/Blueprints/FPSDemo/MT_RedKey.MT_RedKey"))
      (:`NewEnumerator1`
        (`PrimitiveComponent.SetMaterial` _door 0 "/Game/Blueprints/FPSDemo/MT_BlueKey.MT_BlueKey"))
      (:`NewEnumerator2`
        (`PrimitiveComponent.SetMaterial` _door 0 "/Game/Blueprints/FPSDemo/MT_YellowKey.MT_YellowKey")))))